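; Dungeon Blueprint that builds a tile-based level from the InitialLayout data table on BeginPlay.
; LoadInitialLayout copies each table row into CurrentLayout, then InstantiateActors spawns a Block, Wall or Goal actor for each entry by its type.
; PositionToTransform converts a flat tile index into a world location on a flat, ten-column grid with 100-unit spacing.
; The same load and spawn calls sit disconnected in the construction script.
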(event `self.ReceiveBeginPlay`
  (`self.Load Initial Layout`)
  (`self.Instantiate Actors`))

(fn `Instantiate Actors`
  (for _array_element (`self.Current Layout`)
    (bind (_position _type) (break `/Game/Blueprints/Tile` _array_element))
    (bind _transform (`self.Position to Transform` _position))
    (`self.Spawn from Tile Contents` _type _transform)))

(fn `Load Initial Layout`
  (bind _outrownames (`DataTableFunctionLibrary.GetDataTableRowNames` (`self.Initial Layout`)))
  (for _array_element _outrownames
    (bind _returnvalue (`|GetDataTableRow` (`self.Initial Layout`) _array_element)
      (:`then`
        (`KismetArrayLibrary.Array_Add` (`self.Current Layout`) _returnvalue)))))

(fn `Position to Transform`
  (params (Position :type Integer))
  (returns (Transform :type "Transform Structure"))
  (return (`KismetMathLibrary.MakeTransform` (* (`KismetMathLibrary.MakeVector` (`KismetMathLibrary.Conv_IntToDouble` (mod Position 10)) (`KismetMathLibrary.Conv_IntToDouble` (/ Position 10))) 100))))

(fn `Spawn from Tile Contents`
  (params (`Tile Contents` :type "/Game/Blueprints/TileContents Enum" :default "NewEnumerator0") (Location :type "Transform Structure"))
  (switch `/Game/Blueprints/TileContents` `Tile Contents`
    (:`NewEnumerator2`
      (`|SpawnActorFromClass` "/Game/Blueprints/Block.Block_C" Location "Undefined" "OverrideRootScale" null null))
    (:`NewEnumerator3`
      (`|SpawnActorFromClass` "/Game/Blueprints/Wall.Wall_C" Location "Undefined" "OverrideRootScale" null null))
    (:`NewEnumerator4`
      (`|SpawnActorFromClass` "/Game/Blueprints/Goal.Goal_C" Location "Undefined" "OverrideRootScale" null null))))

(fn `UserConstructionScript`)