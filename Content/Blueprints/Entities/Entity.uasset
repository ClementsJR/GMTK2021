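; Entity actor that tracks its X and Y coordinates on a tile grid and moves in tile steps.
; Set Tile Data derives the coordinates from a linear tile position on a 10-wide grid, without moving the actor.
; Update XY adds an offset to the coordinates, then Update Location shifts the actor by 100 units per tile without sweeping, keeping its height.
; Get XY returns the coordinates; the event graph is empty.
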(fn `Get XY`
  (returns (X :type Integer) (Y :type Integer))
  (return (`self.X`) (`self.Y`)))

(fn `Set Tile Data`
  (params (`Tile Data` :type "/Game/Blueprints/Tile_Data Structure"))
  (bind _position (break `/Game/Blueprints/Tile_Data` `Tile Data`))
  (set `self.X` (mod _position 10))
  (set `self.Y` (/ _position 10)))

(fn `Update Location`
  (params (`X Offset` :type Integer) (`Y Offset` :type Integer))
  (`self.K2_SetActorLocation` (`KismetMathLibrary.MakeVector` (+ (* `X Offset` 100.0) (.x (`self.K2_GetActorLocation`))) (+ (* `Y Offset` 100.0) (.y (`self.K2_GetActorLocation`))) (.z (`self.K2_GetActorLocation`)))))

(fn `Update XY`
  (params (`X Offset` :type Integer) (`Y Offset` :type Integer))
  (set `self.X` (+ `X Offset` (`self.X`)))
  (set `self.Y` (+ `Y Offset` (`self.Y`)))
  (`self.Update Location` (`local.X Offset`) (`local.Y Offset`)))

(fn `UserConstructionScript`)