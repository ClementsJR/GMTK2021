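; MobileEntity is a Blueprint base for grid-based entities that slide smoothly between tiles.
; UpdateXY shifts the grid X/Y by an offset and sets a world target at 100 units per cell, keeping Z.
; While moving, Tick accumulates time and MoveTowardTarget lerps from start to target over MaxMoveTime, without sweep, then stops.
; UpdateLocation is an empty stub.
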(event `self.ReceiveTick`
  (params (DeltaSeconds :type "Float (single-precision)"))
  (if (`self.Is Moving`)
    (set `self.Move Time` (+ DeltaSeconds (`self.Move Time`)))
    (`self.Move Toward Target`)))

(fn `Move Toward Target`
  (`self.K2_SetActorLocation` (`KismetMathLibrary.VLerp` (`self.Current Position`) (`self.Target Position`) (`KismetMathLibrary.FClamp` (/ (`self.Move Time`) (`self.Max Move Time`)))))
  (set `self.Is Moving` (not (>= (`self.Move Time`) (`self.Max Move Time`)))))

(fn `Update Location`
  (params (`X Offset` :type Integer) (`Y Offset` :type Integer)))

(fn `Update XY`
  (params (`X Offset` :type Integer) (`Y Offset` :type Integer))
  (set `self.Target Position` (`KismetMathLibrary.MakeVector` (+ (* `X Offset` 100.0) (.x (`self.K2_GetActorLocation`))) (+ (* `Y Offset` 100.0) (.y (`self.K2_GetActorLocation`))) (.z (`self.K2_GetActorLocation`))))
  (set `self.Current Position` (`self.K2_GetActorLocation`))
  (set `self.Move Time` 0.0)
  (set `self.Is Moving` true)
  (set `self.X` (+ (`self.X`) (`local.X Offset`)))
  (set `self.Y` (+ (`self.Y`) (`local.Y Offset`))))

(fn `UserConstructionScript`
  (`parent.UserConstructionScript`))