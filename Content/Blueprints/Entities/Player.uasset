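; Player entity Blueprint with a Mouse mesh that turns to face the direction of its XY offset moves and animates walking.
; BeginPlay caches the Player_Animations instance, and Tick passes the parent's IsMoving state into its IsWalking flag.
; UpdateXY snaps yaw using arccos of X, or arcsin of Y when X is zero, shifted by -90 degrees, then defers to the parent.
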(event `self.ReceiveBeginPlay`
  (bind _asplayer_animations (cast `/Game/Assets/Player/Animations/Player_Animations` (`SkeletalMeshComponent.GetAnimInstance` (`self.Mouse`))))
  (set `self.Animation Controller` _asplayer_animations))

(event `self.ReceiveTick`
  (params (DeltaSeconds :type "Float (single-precision)"))
  (`parent.ReceiveTick` DeltaSeconds)
  (set `/Game/Assets/Player/Animations/Player_Animations.Is Walking` (`self.Is Moving`) (`self.Animation Controller`)))

(fn `Update XY`
  (params (`X Offset` :type Integer) (`Y Offset` :type Integer))
  (if (!= `X Offset` 0)
    (`self.K2_SetActorRotation` (`KismetMathLibrary.MakeRotator` 0.0 0.0 (+ (`KismetMathLibrary.DegAcos` (`KismetMathLibrary.Conv_IntToDouble` `X Offset`)) -90.0)))
    (else
      (`self.K2_SetActorRotation` (`KismetMathLibrary.MakeRotator` 0.0 0.0 (+ (`KismetMathLibrary.DegAsin` (`KismetMathLibrary.Conv_IntToDouble` `Y Offset`)) -90.0)))))
  (`parent.Update XY` (`local.X Offset`) (`local.Y Offset`)))

(fn `UserConstructionScript`)