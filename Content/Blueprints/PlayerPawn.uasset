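; Player pawn that moves its TempBody component in fixed steps on the world X/Y plane from directional input.
; Each Up, Down, Left or Right press calls Move with a 100-unit offset, with horizontal on X and vertical on Y (Up is negative).
; Move adds the offset to the component's world location without sweeping, so the step is instant and ignores collision along the path.
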(event `InputAction|Up`
  (params (Key :type "Key Structure"))
  (:`Pressed`
    (`self.Move` 0 -100)))

(event `InputAction|Right`
  (params (Key :type "Key Structure"))
  (:`Pressed`
    (`self.Move` 100)))

(event `InputAction|Down`
  (params (Key :type "Key Structure"))
  (:`Pressed`
    (`self.Move` 0 100)))

(event `InputAction|Left`
  (params (Key :type "Key Structure"))
  (:`Pressed`
    (`self.Move` -100)))

(fn `Move`
  (params (Horizontal :type Integer) (Vertical :type Integer))
  (`SceneComponent.K2_SetWorldLocation` (`self.Temp Body`) (+ (`KismetMathLibrary.MakeVector` (`KismetMathLibrary.Conv_IntToDouble` Horizontal) (`KismetMathLibrary.Conv_IntToDouble` Vertical)) (`SceneComponent.K2_GetComponentLocation` (`self.Temp Body`))) false false)
  (return))

(fn `UserConstructionScript`)