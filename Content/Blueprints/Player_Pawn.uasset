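; Player pawn that acts as the input relay for a Dungeon actor, which receives all movement and reset requests.
; On BeginPlay it finds the Dungeon with GetActorOfClass and caches the reference.
; Up, Right, Down and Left action presses call PlayerMove with a direction enum, and the Reset action calls the Dungeon's Reset.
; The pawn holds no movement logic of its own.
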(event `self.ReceiveBeginPlay`
  (bind _returnvalue (`GameplayStatics.GetActorOfClass` "/Game/Blueprints/Dungeon.Dungeon_C"))
  (set `self.Dungeon Reference` _returnvalue))

(event `InputAction|Up`
  (params (Key :type "Key Structure"))
  (:`Pressed`
    (`/Game/Blueprints/Dungeon.Player Move` (`self.Dungeon Reference`) "NewEnumerator0")))

(event `InputAction|Right`
  (params (Key :type "Key Structure"))
  (:`Pressed`
    (`/Game/Blueprints/Dungeon.Player Move` (`self.Dungeon Reference`) "NewEnumerator1")))

(event `InputAction|Down`
  (params (Key :type "Key Structure"))
  (:`Pressed`
    (`/Game/Blueprints/Dungeon.Player Move` (`self.Dungeon Reference`) "NewEnumerator2")))

(event `InputAction|Left`
  (params (Key :type "Key Structure"))
  (:`Pressed`
    (`/Game/Blueprints/Dungeon.Player Move` (`self.Dungeon Reference`) "NewEnumerator3")))

(event `InputAction|Reset`
  (params (Key :type "Key Structure"))
  (:`Pressed`
    (`/Game/Blueprints/Dungeon.Reset` (`self.Dungeon Reference`))))

(fn `UserConstructionScript`)